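; Player controller for a cabin-in-the-woods game that sets up input and HUD and times the onset of a blizzard.
; BeginPlay caches the player character, adds the default Enhanced Input mapping context, and creates the log counter and pointer widgets.
; Tick counts BlizzardTime down and, once it runs out, sets IsBlizzard and calls StartBlizzard on the character a single time.
; UpdateLogs forwards log counts to the counter widget.
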(event EventBeginPlay
  (Utilities|FlowControl|Sequence
    (:then_0
      (bind _asbp_player_character (Utilities|Casting|CastToBP_PlayerCharacter (Game|Player|GetPlayerPawn 0)))
      (Variables|Default|SetPlayerCharacter _asbp_player_character))
    (:then_1
      (CallFunction|AddMappingContext "/Game/CabinInTheWoods/Core/Input/IMC_Default.IMC_Default"))
    (:then_2
      (bind _returnvalue (UserInterface|CreateWidget "/Game/CabinInTheWoods/Blueprints/Widgets/W_LogCount.W_LogCount_C" self))
      (bind _output_get (Variables|Default|SetLogUI _returnvalue))
      (UserInterface|Viewport|AddtoViewport _output_get 0)
      (Default|UpdateLogs _output_get))
    (:then_3
      (bind _returnvalue_2 (UserInterface|CreateWidget "/Game/CabinInTheWoods/Blueprints/Widgets/W_Pointer.W_Pointer_C" self))
      (bind _output_get_2 (Variables|Default|SetPointerUI _returnvalue_2))
      (UserInterface|Viewport|AddtoViewport _output_get_2 0))))

(event EventTick
  (params (DeltaSeconds :type Float%20%28single-precision%29))
  (if (not (Variables|Default|GetbIsBlizzard))
    (bind _output_get (Variables|Default|SetBlizzardTime (- (Variables|Default|GetBlizzardTime) DeltaSeconds)))
    (if (<= _output_get 0.0)
      (Variables|Default|SetbIsBlizzard true)
      (Default|StartBlizzard (Variables|Default|GetPlayerCharacter)))))

(fn ConstructionScript)

(fn AddMappingContext
  (params (MappingContext :type Input%20Mapping%20Context%20Object%20Reference) (Priority :type Integer))
  (Input|AddMappingContext (PlayerController|LocalPlayerSubsystems|GetEnhancedInputLocalPlayerSubsystem self) MappingContext Priority "(bIgnoreAllPressedKeysUntilRelease=True,bForceImmediately=False)"))

(fn UpdateLogs
  (params (LogCount :type Integer))
  (Default|UpdateLogs (Variables|Default|GetLogUI) LogCount))