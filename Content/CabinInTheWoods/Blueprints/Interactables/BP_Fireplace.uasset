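; BP_Fireplace is an interactable fireplace that the player fills with carried logs to end the game.
; On interaction, it takes logs from BP_PlayerCharacter and snaps each to the next static mesh socket, whose names are gathered at BeginPlay.
; Once every socket is filled, it activates the fire particles, plays the crackling sound and calls FinishGame on BP_PlayerController.
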(event EventBeginPlay
  (Variables|Default|SetSlotNames (Transformation|GetAllSocketNames (Variables|Default|GetStaticMesh))))

(event Collision|EventActorBeginOverlap
  (params (OtherActor :type Actor%20Object%20Reference)))

(event EventTick
  (params (DeltaSeconds :type Float%20%28single-precision%29)))

(event EventInteract
  (bind _asbp_player_character (Utilities|Casting|CastToBP_PlayerCharacter (Game|Player|GetPlayerPawn 0)))
  (CallFunction|PlaceLogs _asbp_player_character))

(event EventInteractwith
  (bind _asbp_player_character (Utilities|Casting|CastToBP_PlayerCharacter (Game|Player|GetPlayerPawn 0)))
  (CallFunction|PlaceLogs _asbp_player_character))

(fn ConstructionScript)

(fn PlaceLogs
  (params (Player :type BP%20Player%20Character%20Object%20Reference))
  (while (and (Variables|/Game/CabinInTheWoods/Core/Player/BP_PlayerCharacter.BP_PlayerCharacter_C|GetbHasLogs Player) (< (Variables|Default|GetLogs) (Utilities|Array|Length (Variables|Default|GetSlotNames))))
    (bind _log (Default|PlaceLog Player))
    (Transformation|AttachComponentToComponent _log (Variables|Default|GetStaticMesh) (Utilities|Array|Get(acopy) (Variables|Default|GetSlotNames) (Variables|Default|GetLogs)) "SnapToTarget" "SnapToTarget" "KeepWorld" true)
    (Math|Integer|IncrementInt (Variables|Default|GetLogs)))
  (if (== (Variables|Default|GetLogs) (Utilities|Array|Length (Variables|Default|GetSlotNames)))
    (Components|Activation|Activate (Variables|Default|GetP_Fire) false)
    (Audio|Components|Audio|Play (Variables|Default|GetFireCrackling) 0.0)
    (bind _asbp_player_controller (Utilities|Casting|CastToBP_PlayerController (Game|GetPlayerController 0)))
    (Default|FinishGame _asbp_player_controller)))