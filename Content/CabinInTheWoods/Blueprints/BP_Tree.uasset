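; BP_Tree is a choppable tree actor that turns into a log.
; On BeginPlay it picks a random DT_Trees row to set its standing mesh.
; Each ChopTree call lowers Health and plays WoodChop, swapping to that row's fallen mesh and material when Health runs out.
; A further chop on the fallen tree spawns BP_Log at its location, plays WoodSplit and destroys the tree.
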(event EventBeginPlay
  (bind _outrownames (DataTable|GetDataTableRowNames "/Game/CabinInTheWoods/Resources/DataTables/Trees/DT_Trees.DT_Trees"))
  (bind _returnvalue (Utilities|GetDataTableRow "/Game/CabinInTheWoods/Resources/DataTables/Trees/DT_Trees.DT_Trees" (.OutItem (Utilities|Array|Random _outrownames)))
    (:then
      (bind _output_get (Variables|Default|SetTreeInfo _returnvalue))
      (Components|StaticMesh|SetStaticMesh (Variables|Default|GetStaticMesh) (.StandingTree (Utilities|Struct|BreakS_Tree _output_get))))))

(fn ConstructionScript)

(fn ChopTree
  (bind _health (Variables|Default|GetHealth))
  (bind _staticmesh (Variables|Default|GetStaticMesh))
  (bind _treeinfo (Variables|Default|GetTreeInfo))
  (bind (_standingtree _fallentree _basematerial _basefallenmaterial) (Utilities|Struct|BreakS_Tree _treeinfo))
  (if (<= (Variables|Default|GetHealth) 0)
    (Game|SpawnActorfromClass "/Game/CabinInTheWoods/Blueprints/Interactables/BP_Log.BP_Log_C" (Math|Transform|MakeTransform (Transformation|GetActorLocation) "0, 0, 0" "1.000000,1.000000,1.000000") "Undefined" "MultiplyWithRoot" 0 0)
    (Audio|Components|Audio|Play (Variables|Default|GetWoodSplit) 0.0)
    (Actor|DestroyActor)
    (else
      (Math|Integer|DecrementInt _health
        (:%20%20
          (Audio|Components|Audio|Play (Variables|Default|GetWoodChop) 0.0)
          (if (<= _health 0)
            (Components|StaticMesh|SetStaticMesh _staticmesh _fallentree)
            (Rendering|Material|SetMaterial _staticmesh 0 _basefallenmaterial)))))))